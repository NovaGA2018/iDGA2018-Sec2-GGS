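; BP_Enemy is a chasing enemy for a top-down shooter that ends the player's run when it reaches them.
; When PawnSensing sees the player pawn, it uses AI MoveTo to pursue it and reloads the map by opening the level by name on success.
; A DamageHealth event subtracts DamageAmount from Health, and a delayed Tick check destroys the actor once Health runs out.
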(event `self.PawnSensing.OnSeePawn`
  (params (Pawn :type "Pawn Object Reference"))
  (bind _astop_down_shooter_pawn_with_mouse_turning_and_movement (cast `/Game/TwinStickCPP/TopDownShooterPawnWithMouseTurningAndMovement` Pawn))
  (`|AIMoveTo` self (0.0 0.0 0.0) _astop_down_shooter_pawn_with_mouse_turning_and_movement
    (:`OnSuccess`
      (`GameplayStatics.OpenLevel` "Actual_Map_Do_Not_Mess_With_Please"))))

(event `self.ReceiveTick`
  (params (DeltaSeconds :type "Float (single-precision)"))
  (`KismetSystemLibrary.Delay` 0.2)
  (if (<= (`self.Health`) 0.0)
    (`self.ActorDeath`)))

(event `ActorDeath`
  (`self.K2_DestroyActor`))

(event `DamageHealth`
  (set `self.Health` (- (`self.Health`) (`self.DamageAmount`))))

(fn `UserConstructionScript`)